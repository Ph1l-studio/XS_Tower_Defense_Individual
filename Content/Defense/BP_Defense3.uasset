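; BP_Defense3 is a defense turret that turns toward Enemy-tagged actors and fires BP_Bullet until destroyed by damage.
; DetectionRange, a sphere sized in construction, sets the target on overlap and seeks another when it leaves.
; A fast looping timer drives aiming, with a BulletSpeed Delay throttling shots; AcquireNextTarget's own timer has no event shown.
; TakeDamage updates the WBP_DefenseHealth widget and destroys the actor at zero health.
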(event OnComponentBeginOverlap(detectionRange)
  (params (OverlappedComponent :type Primitive%20Component%20Object%20Reference) (OtherActor :type Actor%20Object%20Reference) (OtherComp :type Primitive%20Component%20Object%20Reference) (OtherBodyIndex :type Integer) (bFromSweep :type Boolean) (SweepResult :type Hit%20Result%20Structure%20%28by%20ref%29))
  ;[0.15 0.15 0.15 0.5] Zone Where Defense looks at you and fire
  (Utilities|String|LogString "HIT")
  (if (Actor|ActorHasTag OtherActor "Enemy")
    (CallFunction|LookingatTarget OtherActor)))

(event OnComponentEndOverlap(detectionRange)
  (params (OverlappedComponent :type Primitive%20Component%20Object%20Reference) (OtherActor :type Actor%20Object%20Reference) (OtherComp :type Primitive%20Component%20Object%20Reference) (OtherBodyIndex :type Integer))
  ;[0.15 0.15 0.15 0.5] Zone Where Defense looks at you and fire
  (if (== OtherActor (Variables|Default|GetCurrentTarget))
    (Utilities|Time|ClearandInvalidateTimerbyHandle (Variables|Default|GetTimerLookAt))
    (Variables|Default|SetTimerLookAt "")
    (Variables|Default|SetCurrentTarget 0)
    (CallFunction|AcquireNextTarget)))

(event Custom|LookingAtTarget
  (params (Actor :type Actor%20Object%20Reference))
  (if (Actor|ActorHasTag Actor "Enemy")
    (bind _output_get (Variables|Default|SetCurrentTarget Actor))
    (bind _returnvalue (Utilities|Time|SetTimerbyEvent (delegate Custom|LookTimer) 0.03 true))
    (Variables|Default|SetTimerLookAt _returnvalue)))

(event Custom|LookTimer
  (Utilities|IsValid (stale Custom|LookingAtTarget _output_get)
    (:Is%20Valid
      (Transformation|SetActorRotation (Math|Rotator|MakeRotator 0.0 (.pitch (Math|Rotator|FindLookatRotation (Transformation|GetActorLocation) (Transformation|GetActorLocation (stale Custom|LookingAtTarget _output_get)))) (.yaw (Math|Rotator|FindLookatRotation (Transformation|GetActorLocation) (Transformation|GetActorLocation (stale Custom|LookingAtTarget _output_get))))))
      (Utilities|FlowControl|Delay (Variables|Default|GetBulletSpeed))
      (Game|SpawnActorfromClass "/Game/Defense/BP_Bullet.BP_Bullet_C" (Transformation|GetWorldTransform (Variables|Default|GetBullet)) "Undefined" "MultiplyWithRoot" 0 0))
    (:Is%20Not%20Valid
      (CallFunction|AcquireNextTarget))))

(event Custom|TakeDamage
  (params (Amount :type Float%20%28double-precision%29))
  (Variables|Default|SetCurrentHealth (- (Variables|Default|GetCurrentHealth) Amount))
  (bind _aswbp_defense_health (Utilities|Casting|CastToWBP_DefenseHealth (UserInterface|GetUserWidgetObject (Variables|Default|GetHealthWidget))))
  (Default|SetHealthPercent _aswbp_defense_health (/ (Variables|Default|GetCurrentHealth) (Variables|Default|GetMaxHealth)))
  (if (<= (Variables|Default|GetCurrentHealth) 0.0)
    (Utilities|Time|ClearandInvalidateTimerbyHandle (Variables|Default|GetTimerLookAt))
    (Actor|DestroyActor)))

(event Custom|AcquireNextTarget
  (Utilities|IsValid (Variables|Default|GetCurrentTarget)
    (:Is%20Not%20Valid
      (for _array_element (Collision|GetOverlappingActors (Components|GetOwner (Variables|Default|GetdetectionRange)) 0 :!class /Script/Engine.Actor)
        (if (Actor|ActorHasTag _array_element "Enemy")
          (Variables|Default|SetCurrentTarget _array_element)
          (bind _returnvalue (Utilities|Time|SetTimerbyEvent 0 0.05 true))
          (Variables|Default|SetTimerLookAt _returnvalue)
          (Utilities|FlowControl|ForLoopwithBreak 0 0) ; enters at Break
        )))))

(event EventBeginPlay
  (Variables|Default|SetCurrentHealth (Variables|Default|GetMaxHealth))
  (Utilities|FlowControl|Delay 0.1)
  (for _array_element (Collision|GetOverlappingActors (Components|GetOwner (Variables|Default|GetdetectionRange)) "/Game/Blueprints/BP_Mummy.BP_Mummy_C" :!class /Script/Engine.Actor)
    (bind _asbp_mummy (Utilities|Casting|CastToBP_Mummy _array_element))
    (Variables|Default|SetCurrentTarget 0)
    (Transformation|SetActorRotation (Math|Rotator|FindLookatRotation (Transformation|GetActorLocation _asbp_mummy) (Transformation|GetActorLocation)))
    (Utilities|FlowControl|ForLoopwithBreak 0 0) ; enters at Break
  ))

(fn ConstructionScript
  (Components|Sphere|SetSphereRadius (Variables|Default|GetdetectionRange) (Variables|Default|GetIn%20Sphere%20Radius) true))