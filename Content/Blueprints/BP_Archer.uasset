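; Ranged enemy that walks a path toward the tower, shooting on the move, and destroys itself at the last point.
; SetupArcher supplies path and tower; Tick steers between points and fires BP_ArcherArrow on cooldown at the first BP_Defense in range, otherwise the tower at any distance.
; AnyDamage updates the health widget, while ReceiveDamage resets it to full; both can trigger Die, which registers the kill.
; Melee attack and BP_Arrow logic is disconnected.
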(event Custom|DealDamage)

(event Custom|StartAttack)

(event Custom|Die
  (Variables|Default|SetbDead true)
  (Utilities|Time|ClearandInvalidateTimerbyHandle (Variables|Default|GetAttackTimer))
  (bind _asbp_tower (Utilities|Casting|CastToBP_Tower (Variables|Default|GetTower)))
  (Default|RegisterKill _asbp_tower (Transformation|GetActorLocation))
  (Actor|DestroyActor))

(event Collision|EventActorBeginOverlap
  (params (OtherActor :type Actor%20Object%20Reference)))

(event EventTick
  (params (DeltaSeconds :type Float%20%28single-precision%29))
  (bind _returnvalue (Transformation|GetActorLocation))
  (bind _returnvalue_2 (Transformation|GetActorLocation))
  (if (not (or (Variables|Default|GetbDead) (Variables|Default|GetbReachedEnd)))
    (if (>= (Variables|Default|GetPointIndex) (Utilities|Array|Length (Variables|Default|GetPathPoints)))
      (Variables|Default|SetbReachedEnd true)
      (Actor|DestroyActor)
      (else
        (Transformation|SetActorLocation (+ _returnvalue_2 (* (* (Math|Vector|Normalize (- (Utilities|Array|Get(acopy) (Variables|Default|GetPathPoints) (Variables|Default|GetPointIndex)) (Transformation|GetActorLocation))) (Variables|Default|GetMoveSpeed)) DeltaSeconds)) false false)
        (Transformation|SetActorRotation (Math|Rotator|FindLookatRotation _returnvalue_2 (Utilities|Array|Get(acopy) (Variables|Default|GetPathPoints) (Variables|Default|GetPointIndex))))
        (if (< (Math|Vector|Distance(Vector) (Transformation|GetActorLocation) (Utilities|Array|Get(acopy) (Variables|Default|GetPathPoints) (Variables|Default|GetPointIndex))) 6e+01)
          (Variables|Default|SetPointIndex (+ (Variables|Default|GetPointIndex) 1))
          (elif (<= (Variables|Default|GetFireCooldown) 0.0)
            (Variables|Default|SetShotTarget (Variables|Default|GetTower))
            (bind _outactors (Actor|GetAllActorsOfClass "/Game/Defense/BP_Defense.BP_Defense_C"))
            (bind _array_element (Utilities|Array|ForEachLoopwithBreak _outactors :!label _label)
              (:LoopBody
                (if (< (Math|Vector|Distance(Vector) (Transformation|GetActorLocation _array_element) (Transformation|GetActorLocation)) (Variables|Default|GetShootRange))
                  (Variables|Default|SetShotTarget _array_element)
                  (goto _label Break)))
              (:Completed
                (Utilities|IsValid (Variables|Default|GetShotTarget)
                  (:Is%20Valid
                    (Transformation|SetActorRotation (Math|Rotator|FindLookatRotation _returnvalue (Transformation|GetActorLocation (Variables|Default|GetShotTarget))))
                    (Game|SpawnActorfromClass "/Game/Blueprints/BP_ArcherArrow.BP_ArcherArrow_C" (Math|Transform|MakeTransform _returnvalue (Math|Rotator|FindLookatRotation _returnvalue (Transformation|GetActorLocation (Variables|Default|GetShotTarget)))) "AlwaysSpawn" "MultiplyWithRoot" 0 0)
                    (Variables|Default|SetFireCooldown (Variables|Default|GetFireRate))))))
            (else
              (Variables|Default|SetFireCooldown (- (Variables|Default|GetFireCooldown) DeltaSeconds)))))))))

(event Game|Damage|EventAnyDamage
  (params (Damage :type Float%20%28single-precision%29) (DamageType :type Damage%20Type%20Object%20Reference) (InstigatedBy :type Controller%20Object%20Reference) (DamageCauser :type Actor%20Object%20Reference))
  (Variables|Default|SetCurrentHealth (- (Variables|Default|GetCurrentHealth) Damage))
  (bind _aswbp_archer_health (Utilities|Casting|CastToWBP_ArcherHealth (UserInterface|GetUserWidgetObject (Variables|Default|GetWidget))))
  (Default|SetHealthPercent _aswbp_archer_health (/ (Variables|Default|GetCurrentHealth) (Variables|Default|GetMaxHealth)))
  (if (<= (Variables|Default|GetCurrentHealth) 0.0)
    (CallFunction|Die)))

(event EventBeginPlay
  (Variables|Default|SetCurrentHealth (Variables|Default|GetMaxHealth)))

(fn ConstructionScript)

(fn SetupArcher
  (params (InPoints :type Array%20of%20Vectors) (InTower%20 :type Actor%20Object%20Reference))
  (Variables|Default|SetPathPoints InPoints)
  (Variables|Default|SetTower InTower%20)
  (Variables|Default|SetAttackTarget 0)
  (Variables|Default|SetCurrentHealth (Variables|Default|GetMaxHealth))
  (Variables|Default|SetPointIndex 0)
  (Variables|Default|SetbReachedEnd false)
  (Components|Animation|PlayAnimation (Variables|Default|GetArcher) "/Game/Characters/Archer/Standing_Aim_Walk_Forward_Anim.Standing_Aim_Walk_Forward_Anim" true)
  (Variables|Default|SetbDead false)
  (Transformation|SetActorLocation (Utilities|Array|Get(acopy) (Variables|Default|GetPathPoints)) false false)
  (bind _aswbp_archer_health (Utilities|Casting|CastToWBP_ArcherHealth (UserInterface|GetUserWidgetObject (Variables|Default|GetWidget))))
  (Default|SetHealthPercent _aswbp_archer_health 1.0)
  (Transformation|SetActorRotation (Math|Rotator|FindLookatRotation (Transformation|GetActorLocation) (Transformation|GetActorLocation (Variables|Default|GetTower)))))

(fn ReceiveDamage
  (params (Amount :type Float%20%28double-precision%29))
  (Variables|Default|SetCurrentHealth (- (Variables|Default|GetCurrentHealth) Amount))
  (bind _aswbp_archer_health (Utilities|Casting|CastToWBP_ArcherHealth (UserInterface|GetUserWidgetObject (Variables|Default|GetWidget))))
  (Default|SetHealthPercent _aswbp_archer_health 1.0)
  (if (<= (Variables|Default|GetCurrentHealth) 0.0)
    (CallFunction|Die)))