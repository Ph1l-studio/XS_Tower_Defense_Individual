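; BP_Tower is the defended tower, which tracks health, triggers game over and rewards kills with gems.
; On BeginPlay it fills its health, creates the W_HUD widget and calls its MiningDefense function.
; ReceiveDamage updates the HUD health percent and, at zero health, shows W_GameOver with the cursor and UI-only input.
; RegisterKill counts kills and, at each KillsPerGem threshold, spawns a gem above the supplied location.
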(event EventBeginPlay
  (Variables|Default|SetCurrentHealth (Variables|Default|GetMaxHealth))
  (bind _returnvalue (UserInterface|CreateWidget "/Game/UI/W_HUD.W_HUD_C"))
  (bind _output_get (Variables|Default|SetTowerHealthWidget _returnvalue))
  (UserInterface|Viewport|AddtoViewport _output_get 0)
  (Default|SetHealthPercent (Variables|Default|GetTowerHealthWidget) 1.0)
  (Variables|/Game/UI/W_HUD.W_HUD_C|SetTowerRef (Variables|Default|GetTowerHealthWidget) 0)
  (Default|MiningDefense (Variables|Default|GetTowerHealthWidget)))

(fn ConstructionScript)

(fn ReceiveDamage
  (params (Amount :type Float%20%28double-precision%29))
  (bind _returnvalue (Game|GetPlayerController 0))
  (Variables|Default|SetCurrentHealth (- (Variables|Default|GetCurrentHealth) Amount))
  (Default|SetHealthPercent (Variables|Default|GetTowerHealthWidget) (/ (Variables|Default|GetCurrentHealth) (Variables|Default|GetMaxHealth)))
  (if (<= (Variables|Default|GetCurrentHealth) 0.0)
    (Variables|Default|SetbDead false)
    (bind _returnvalue_2 (UserInterface|CreateWidget "/Game/UI/W_GameOver.W_GameOver_C"))
    (UserInterface|Viewport|AddtoViewport _returnvalue_2 0)
    (Variables|/Script/Engine.PlayerController|SetbShowMouseCursor _returnvalue true)
    (Input|SetInputModeUIOnly _returnvalue 0 "DoNotLock" false)))

(fn RegisterKill
  (params (SpawnLocation :type Vector))
  (Variables|Default|SetKillCount (+ (Variables|Default|GetKillCount) 1))
  (if (>= (Variables|Default|GetKillCount) (Variables|Default|GetKillsPerGem))
    (Variables|Default|SetKillCount 0)
    (Game|SpawnActorfromClass (Variables|Default|GetGemClass) (Math|Transform|MakeTransform (+ SpawnLocation (Math|Vector|MakeVector 0.0 0.0 8e+01))) "AlwaysSpawn" "MultiplyWithRoot" 0 0)
    (Development|PrintText "Gem Spawned")))