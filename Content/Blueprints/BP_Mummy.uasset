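; Tower-defense enemy mummy that walks a point path supplied by SetupMummy toward the Tower, attacking defenses it meets.
; Each Tick it scans all BP_Defense actors by distance, moves along the path, and stops to attack a nearby defense or the tower at the path's end.
; A looping timer deals the damage.
; Incoming damage updates a health widget; death reports the kill to BP_Tower and destroys the actor.
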(event Custom|DealDamage
  (bind _attackdamage (Variables|Default|GetAttackDamage))
  (Utilities|IsValid (Variables|Default|GetAttackTarget)
    (:Is%20Valid
      (bind _asbp_defense (Utilities|Casting|CastToBP_Defense (Variables|Default|GetAttackTarget))
        (:then
          (Default|TakeDamage _asbp_defense _attackdamage))
        (:CastFailed
          (bind _asbp_tower (Utilities|Casting|CastToBP_Tower (Variables|Default|GetTower)))
          (Default|ReceiveDamage _asbp_tower _attackdamage))))
    (:Is%20Not%20Valid
      (Components|Animation|PlayAnimation (Variables|Default|GetMummy) "/Game/Characters/Mummy/Running.Running" true)
      (Variables|Default|SetAttackTarget (Variables|Default|GetTower))
      (Variables|Default|SetbReachedEnd false)
      (Utilities|Time|ClearandInvalidateTimerbyHandle (Variables|Default|GetAttackTimer)))))

(event Custom|StartAttack
  (Variables|Default|SetbReachedEnd true)
  (Transformation|SetActorRotation (Math|Rotator|FindLookatRotation (Transformation|GetActorLocation) (Transformation|GetActorLocation (Variables|Default|GetAttackTarget))))
  (bind _returnvalue (Utilities|Time|SetTimerbyEvent (delegate Custom|DealDamage) (Variables|Default|GetAttackInterval) true))
  (Variables|Default|SetAttackTimer _returnvalue))

(event Custom|Die
  (Variables|Default|SetbDead true)
  (Utilities|Time|ClearandInvalidateTimerbyHandle (Variables|Default|GetAttackTimer))
  (bind _asbp_tower (Utilities|Casting|CastToBP_Tower (Variables|Default|GetTower)))
  (Default|RegisterKill _asbp_tower (Transformation|GetActorLocation))
  (Actor|DestroyActor))

(event Collision|EventActorBeginOverlap
  (params (OtherActor :type Actor%20Object%20Reference)))

(event EventTick
  (params (DeltaSeconds :type Float%20%28single-precision%29))
  (bind _returnvalue (Transformation|GetActorLocation))
  (bind _outactors (Actor|GetAllActorsOfClass "/Game/Defense/BP_Defense.BP_Defense_C"))
  (for _array_element _outactors
    (if (< (Math|Vector|Distance(Vector) (Transformation|GetActorLocation) (Transformation|GetActorLocation _array_element)) (Variables|Default|GetDefenseDetectRange))
      (Utilities|IsValid (Variables|Default|GetAttackTarget)
        (:Is%20Not%20Valid
          (Variables|Default|SetAttackTarget _array_element)
          (CallFunction|StartAttack)
          (if (!= (Variables|Default|GetbReachedEnd) (Variables|Default|GetbWasAttacking))
            (Components|Animation|PlayAnimation (Variables|Default|GetMummy) "/Game/Characters/Mummy/Zombie_Attack.Zombie_Attack" true)
            (Variables|Default|SetbWasAttacking (Variables|Default|GetbReachedEnd))
            (else
              (Components|Animation|PlayAnimation (Variables|Default|GetMummy) "/Game/Characters/Mummy/Running.Running" true)))))))
  (if (not (or (Variables|Default|GetbDead) (Variables|Default|GetbReachedEnd)))
    (if (>= (Variables|Default|GetPointIndex) (Utilities|Array|Length (Variables|Default|GetPathPoints)))
      (Variables|Default|SetAttackTarget (Variables|Default|GetTower))
      (CallFunction|StartAttack)
      (Components|Animation|PlayAnimation (Variables|Default|GetMummy) "/Game/Characters/Mummy/Zombie_Attack.Zombie_Attack" true)
      (Variables|Default|SetbWasAttacking (Variables|Default|GetbReachedEnd))
      (else
        (Transformation|SetActorLocation (+ _returnvalue (* (* (Math|Vector|Normalize (- (Utilities|Array|Get(acopy) (Variables|Default|GetPathPoints) (Variables|Default|GetPointIndex)) (Transformation|GetActorLocation))) (Variables|Default|GetMoveSpeed)) DeltaSeconds)) false false)
        (Transformation|SetActorRotation (Math|Rotator|FindLookatRotation _returnvalue (Transformation|GetActorLocation (Variables|Default|GetTower))))
        (if (< (Math|Vector|Distance(Vector) (Transformation|GetActorLocation) (Utilities|Array|Get(acopy) (Variables|Default|GetPathPoints) (Variables|Default|GetPointIndex))) 6e+01)
          (Variables|Default|SetPointIndex (+ (Variables|Default|GetPointIndex) 1)))))))

(event Game|Damage|EventAnyDamage
  (params (Damage :type Float%20%28single-precision%29) (DamageType :type Damage%20Type%20Object%20Reference) (InstigatedBy :type Controller%20Object%20Reference) (DamageCauser :type Actor%20Object%20Reference))
  (Variables|Default|SetCurrentHealth (- (Variables|Default|GetCurrentHealth) Damage))
  (bind _aswbp_mummy_health (Utilities|Casting|CastToWBP_MummyHealth (UserInterface|GetUserWidgetObject (Variables|Default|GetWidget))))
  (Default|SetHealthPercent _aswbp_mummy_health (/ (Variables|Default|GetCurrentHealth) (Variables|Default|GetMaxHealth)))
  (if (<= (Variables|Default|GetCurrentHealth) 0.0)
    (CallFunction|Die)))

(event EventBeginPlay
  (Variables|Default|SetCurrentHealth (Variables|Default|GetMaxHealth)))

(fn ConstructionScript)

(fn SetupMummy
  (params (InPoints :type Array%20of%20Vectors) (InTower%20 :type Actor%20Object%20Reference))
  (Variables|Default|SetPathPoints InPoints)
  (Variables|Default|SetTower InTower%20)
  (Variables|Default|SetAttackTarget 0)
  (Variables|Default|SetCurrentHealth (Variables|Default|GetMaxHealth))
  (Variables|Default|SetPointIndex 0)
  (Variables|Default|SetbReachedEnd false)
  (Components|Animation|PlayAnimation (Variables|Default|GetMummy) "/Game/Characters/Mummy/Running.Running" true)
  (Variables|Default|SetbDead false)
  (Transformation|SetActorLocation (Utilities|Array|Get(acopy) (Variables|Default|GetPathPoints)) false false)
  (bind _aswbp_mummy_health (Utilities|Casting|CastToWBP_MummyHealth (UserInterface|GetUserWidgetObject (Variables|Default|GetWidget))))
  (Default|SetHealthPercent _aswbp_mummy_health 1.0)
  (Transformation|SetActorRotation (Math|Rotator|FindLookatRotation (Transformation|GetActorLocation) (Transformation|GetActorLocation (Variables|Default|GetTower)))))

(fn ReceiveDamage
  (params (Amount :type Float%20%28double-precision%29))
  (Variables|Default|SetCurrentHealth (- (Variables|Default|GetCurrentHealth) Amount))
  (bind _aswbp_mummy_health (Utilities|Casting|CastToWBP_MummyHealth (UserInterface|GetUserWidgetObject (Variables|Default|GetWidget))))
  (Default|SetHealthPercent _aswbp_mummy_health (/ (Variables|Default|GetCurrentHealth) (Variables|Default|GetMaxHealth)))
  (if (<= (Variables|Default|GetCurrentHealth) 0.0)
    (CallFunction|Die)))