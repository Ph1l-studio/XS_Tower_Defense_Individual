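; Player pawn for a tower-defense game that places defenses with the mouse and mines gems.
; BeginPlay creates the HUD linked to the tower and shows the cursor.
; A cursor line trace positions a collisionless mangonel preview each Tick and spawns BP_Defense on left click.
; F increments the tower's gem count for each nearby gem, calls DestroyActor on both gem and tower, then calls the tower widget's MiningDefense.
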(event EventBeginPlay
  (Variables|/Script/Engine.PlayerController|SetbShowMouseCursor (Game|GetPlayerController 0) true)
  (bind _returnvalue (UserInterface|CreateWidget "/Game/UI/W_HUD.W_HUD_C" (Game|GetPlayerController 0)))
  (bind _output_get (Variables|Default|SetHUDRef _returnvalue))
  (bind _outactors (Actor|GetAllActorsOfClass "/Game/Blueprints/BP_Tower.BP_Tower_C"))
  (Variables|/Game/UI/W_HUD.W_HUD_C|SetTowerRef _output_get (Utilities|Array|Get(acopy) _outactors))
  (UserInterface|Viewport|AddtoViewport _output_get 0))

(event EventTick
  (params (DeltaSeconds :type Float%20%28single-precision%29))
  (bind (_returnvalue _outhit) (CallFunction|MouseTrace))
  (if _returnvalue
    (Variables|Default|GetBuild%20Preview
      (:then
        (Transformation|SetWorldLocation (Variables|Default|GetBuild%20Preview) (.Location (Collision|BreakHitResult _outhit)) false false))
      (:else
        (bind _returnvalue_2 (Game|AddComponentbyClass "/Script/Engine.StaticMeshComponent" false (Math|Transform|MakeTransform (.Location (Collision|BreakHitResult _outhit)) "0, 0, 0" "2.000000,2.000000,2.000000")))
        (bind _output_get (Variables|Default|SetBuild%20Preview _returnvalue_2))
        (Components|StaticMesh|SetStaticMesh _output_get "/Game/Fab/Medieval_Mangonel_–_Catapult_Siege_Weapon/010_medieval_mangonel/StaticMeshes/010_medieval_mangonel.010_medieval_mangonel")
        (Collision|SetCollisionEnabled (Variables|Default|GetBuild%20Preview) "NoCollision")
        (Rendering|Material|SetMaterial (Variables|Default|GetBuild%20Preview) 0 "/Game/Fab/Medieval_Mangonel_–_Catapult_Siege_Weapon/010_medieval_mangonel/StaticMeshes/M.M")))))

(event Input|MouseEvents|LeftMouseButton
  (params (Key :type Key%20Structure :default "None"))
  (:Pressed
    (bind (_returnvalue _outhit) (CallFunction|MouseTrace))
    (if _returnvalue
      (Game|SpawnActorfromClass "/Game/Defense/BP_Defense.BP_Defense_C" (Math|Transform|MakeTransform (.Location (Collision|BreakHitResult _outhit)) "0, 0, 0" "2.000000,2.000000,2.000000") "AdjustIfPossibleButAlwaysSpawn" "MultiplyWithRoot" 0 3.5e+03 true 1.0 0))))

(event Input|KeyboardEvents|F
  (params (Key :type Key%20Structure :default "None"))
  (:Pressed
    (bind _outactors (Actor|GetAllActorsOfClass "/Game/Blueprints/BP_Gems.BP_Gems_C"))
    (for _array_element _outactors
      (if true
        (if (< (Math|Vector|Distance(Vector) (Transformation|GetActorLocation) (Transformation|GetActorLocation _array_element)) 4e+02)
          (bind _returnvalue (Actor|GetActorOfClass "/Game/Blueprints/BP_Tower.BP_Tower_C"))
          (Variables|/Game/Blueprints/BP_Tower.BP_Tower_C|SetGems _returnvalue (+ (Variables|/Game/Blueprints/BP_Tower.BP_Tower_C|GetGems _returnvalue) 1))
          (Actor|DestroyActor _returnvalue)
          (Default|MiningDefense (Variables|/Game/Blueprints/BP_Tower.BP_Tower_C|GetTowerHealthWidget _returnvalue)))))))

(fn ConstructionScript)

(fn MouseTrace
  (bind _returnvalue (Game|GetPlayerController 0))
  (bind (_worldlocation _worlddirection) (Game|Player|ConvertMouseLocationToWorldSpace _returnvalue))
  (bind (_outhit _returnvalue_2) (Collision|LineTraceByChannel _worldlocation (+ _worldlocation (* _worlddirection 1e+04)) "TraceTypeQuery1" false 0 "ForDuration"))
  (return _returnvalue_2 _outhit))